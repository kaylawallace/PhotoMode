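; BP_PlayerController is a player controller that toggles a UI Enhanced Input mapping context through its SwitchInputToUI function.
; By default the function adds the UI context at a set priority, leaving input mode and cursor untouched.
; With Reset set, it removes that context, restores game-only input without flushing and hides the mouse cursor.
; The event graph and construction script contain no logic.
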(event EventBeginPlay)

(event EventTick
  (params (DeltaSeconds :type Float%20%28single-precision%29)))

(fn ConstructionScript)

(fn SwitchInputtoUI
  (params (Reset :type Boolean))
  (if Reset
    (Input|RemoveMappingContext (PlayerController|LocalPlayerSubsystems|GetEnhancedInputLocalPlayerSubsystem) (Variables|Default|GetUI_IMC) "(bIgnoreAllPressedKeysUntilRelease=True,bForceImmediately=False)")
    (Input|SetInputModeGameOnly self false)
    (if (Variables|Default|GetbShowMouseCursor)
      (Variables|Default|SetbShowMouseCursor false))
    (else
      (Input|AddMappingContext (PlayerController|LocalPlayerSubsystems|GetEnhancedInputLocalPlayerSubsystem) (Variables|Default|GetUI_IMC) 3 "(bIgnoreAllPressedKeysUntilRelease=True,bForceImmediately=False)"))))