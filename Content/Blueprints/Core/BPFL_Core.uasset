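; Blueprint function library of typed getters for the game's core framework objects: HUD, game instance, player character and player controller.
; Each function casts the engine's generic getter result to the project class and returns it with a Success flag.
; The HUD and character lookups always use player index 0, while the controller getter takes an index.
; The HUD and game instance getters also run a validity check before casting.
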(fn GetHUD
  (params (WorldContext :type Object%20Object%20Reference))
  (bind _returnvalue (Game|GetPlayerController WorldContext))
  (Utilities|IsValid _returnvalue
    (:Is%20Valid
      (bind _asbp_hud (Utilities|Casting|CastToBP_HUD (HUD|GetHUD _returnvalue))
        (:then
          (return true _asbp_hud))
        (:CastFailed
          (return false 0))))
    (:Is%20Not%20Valid
      (return false 0))))

(fn GetGameInstance
  (params (WorldContextObject :type Object%20Object%20Reference))
  (Utilities|IsValid WorldContextObject
    (:Is%20Valid
      (bind _asbp_custom_game_inst (Utilities|Casting|CastToBP_CustomGameInst (Game|GetGameInstance WorldContextObject))
        (:then
          (return true _asbp_custom_game_inst))
        (:CastFailed
          (return false 0))))
    (:Is%20Not%20Valid
      (return false 0))))

(fn GetPlayerCharacter
  (params (WorldContextObject :type Object%20Object%20Reference))
  (bind _asbp_third_person_character (Utilities|Casting|CastToBP_ThirdPersonCharacter (Game|GetPlayerCharacter WorldContextObject))
    (:then
      (return true _asbp_third_person_character))
    (:CastFailed
      (return false 0))))

(fn GetPlayerController
  (params (WorldContextObject :type Object%20Object%20Reference) (PlayerIndex :type Integer))
  (bind _asbp_player_controller (Utilities|Casting|CastToBP_PlayerController (Game|GetPlayerController WorldContextObject PlayerIndex))
    (:then
      (return true _asbp_player_controller))
    (:CastFailed
      (return false 0))))