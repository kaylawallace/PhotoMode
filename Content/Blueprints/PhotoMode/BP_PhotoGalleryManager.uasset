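; Photo mode manager that stores the player's captured photos and drives the gallery UI.
; On BeginPlay it registers itself with the player character.
; New photos are added uniquely to a capped array, silently dropping the oldest when full.
; Toggling the gallery or deleting a photo passes the array to the HUD to show or refresh the gallery.
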(event EventBeginPlay
  (bind (_success _playercharacter) (CallFunction|GetPlayerCharacter))
  (if _success
    (Default|SetPhotoGalleryManager _playercharacter self)))

(fn ConstructionScript)

(fn AddPhototoGallery
  (params (RT_NewPhoto :type Texture%20Render%20Target%202D%20Object%20Reference%20%28by%20ref%29))
  (if (>= (Utilities|Array|Length (Variables|Default|GetPhotoGallery)) (Variables|Default|GetMaxPhotos))
    ;[1 0.1326 0.09279] not the best solution - better: add UI popup and give player option to remove an photo of their choice or discard new photo
    (Utilities|Array|RemoveIndex (Variables|Default|GetPhotoGallery)))
  (Utilities|Array|AddUnique (Variables|Default|GetPhotoGallery) RT_NewPhoto))

(fn TogglePhotoGallery
  (params (Enable :type Boolean))
  (bind (_success _hud) (CallFunction|GetHUD))
  (if _success
    (Default|EnablePhotoGalleryUI _hud Enable (Variables|Default|GetPhotoGallery))))

(fn DeletePhotofromGallery
  (params (PhotoRender :type Texture%20Render%20Target%202D%20Object%20Reference))
  (bind _returnvalue (Utilities|Array|RemoveItem (Variables|Default|GetPhotoGallery) PhotoRender))
  (if _returnvalue
    (bind (_success _hud) (CallFunction|GetHUD))
    (if _success
      (Default|RefreshPhotoGalleryUI _hud (Variables|Default|GetPhotoGallery)))
    (else
      (Development|PrintString "Failed to remove photo from gallery" true true "(R=1.000000,G=0.132596,B=0.092793,A=1.000000)"))))