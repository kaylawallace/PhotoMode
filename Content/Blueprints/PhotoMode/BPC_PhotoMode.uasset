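; Pawn component that adds a photo mode with look, zoom and selfie camera, reusing the owner's camera and spring arm.
; Toggling swaps arm length, input mapping and HUD camera UI; zoom drives FOV, boom height and a detection box.
; The box records IDs of overlapped items in line of sight, never removing them.
; Photos use an on-demand scene capture to a new render target, passed with the gallery manager to HUD confirmation.
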(event Input|EnhancedActionEvents|EnhancedInputActionIA_PhotoModeLook
  (params (ActionValue :type Vector%202D%20Structure) (ElapsedSeconds :type Float%20%28double-precision%29) (TriggeredSeconds :type Float%20%28double-precision%29) (InputAction :type Input%20Action%20Object%20Reference :default "/Game/Blueprints/PhotoMode/Input/Actions/IA_PhotoModeLook.IA_PhotoModeLook"))
  (:Triggered
    (if (Variables|State|GetPhotoModeActive)
      (Movement|MoveCamera ActionValue))))

(event Input|EnhancedActionEvents|EnhancedInputActionIA_TakePhoto
  (params (ActionValue :type Boolean) (ElapsedSeconds :type Float%20%28double-precision%29) (TriggeredSeconds :type Float%20%28double-precision%29) (InputAction :type Input%20Action%20Object%20Reference :default "/Game/Blueprints/PhotoMode/Input/Actions/IA_TakePhoto.IA_TakePhoto"))
  (:Started
    (if (not (Variables|State|GetPhotographyDisabled))
      (Camera|TakePhoto))))

(event Input|EnhancedActionEvents|EnhancedInputActionIA_ToggleSelfieMode
  (params (ActionValue :type Boolean) (ElapsedSeconds :type Float%20%28double-precision%29) (TriggeredSeconds :type Float%20%28double-precision%29) (InputAction :type Input%20Action%20Object%20Reference :default "/Game/Blueprints/PhotoMode/Input/Actions/IA_ToggleSelfieMode.IA_ToggleSelfieMode"))
  (:Started
    (if (not (Variables|State|GetPhotographyDisabled))
      (State|ToggleSelfieMode))))

(event Input|EnhancedActionEvents|EnhancedInputActionIA_CameraZoom
  (params (ActionValue :type Float%20%28double-precision%29) (ElapsedSeconds :type Float%20%28double-precision%29) (TriggeredSeconds :type Float%20%28double-precision%29) (InputAction :type Input%20Action%20Object%20Reference :default "/Game/Blueprints/PhotoMode/Input/Actions/IA_CameraZoom.IA_CameraZoom"))
  (:Triggered
    (Movement|ZoomCamera ActionValue)))

(event EventBeginPlay
  (Component|InitialiseComponent))

(fn InitialiseComponent
  (bind _aspawn (Utilities|Casting|CastToPawn (Components|GetOwner)))
  (bind _output_get (Variables|Owner|SetOwningActor _aspawn))
  (Variables|Default|SetCamera (Actor|GetComponentbyClass _output_get "/Script/Engine.CameraComponent"))
  (Variables|Default|SetSpringArm (Actor|GetComponentbyClass (Variables|Owner|GetOwningActor) "/Script/Engine.SpringArmComponent"))
  (bind _returnvalue (Game|AddComponentbyClass (Variables|Owner|GetOwningActor) "/Script/Engine.SceneCaptureComponent2D" true))
  (bind _output_get_2 (Variables|Default|SetCameraCaptureComponent _returnvalue))
  (Variables|/Script/Engine.SceneCaptureComponent|SetbCaptureEveryFrame _output_get_2 false)
  (Variables|/Script/Engine.SceneCaptureComponent|SetbCaptureOnMovement (Variables|Default|GetCameraCaptureComponent) false)
  (Transformation|AttachComponentToComponent (Variables|Default|GetCameraCaptureComponent) (Variables|Default|GetCamera) "None" "SnapToTarget" "SnapToTarget" "SnapToTarget" true)
  (Component|InitialiseBoxCollision)
  (if (Variables|GalleryManager|GetSpawnGalleryManagerOnBegin)
    (bind _returnvalue_2 (Game|SpawnActorfromClass "/Game/Blueprints/PhotoMode/BP_PhotoGalleryManager.BP_PhotoGalleryManager_C" (Math|Transform|MakeTransform "0, 0, 0" "0, 0, 0" "1.000000,1.000000,1.000000") "Undefined" "MultiplyWithRoot" 0 0))
    (Variables|GalleryManager|SetPhotoGalleryManager _returnvalue_2))
  (Variables|SpringArm|SetDefaultSpringArmLength (Variables|/Script/Engine.SpringArmComponent|GetTargetArmLength (Variables|Default|GetSpringArm)))
  (Variables|SpringArm|SetDefaultSpringArmHeight (.z (Variables|/Script/Engine.SceneComponent|GetRelativeLocation (Variables|Default|GetSpringArm))))
  (Variables|Camera|SetDefaultFOV (Variables|/Script/Engine.CameraComponent|GetFieldOfView (Variables|Default|GetCamera)))
  (bind (_success _hud) (CallFunction|GetHUD self))
  (if _success
    (Variables|UI|SetHUD _hud)))

(fn GetPhotoModeActive
  (return (Variables|State|GetPhotoModeActive)))

(fn GetSelfieModeActive
  (return (Variables|State|GetSelfieModeActive)))

(fn TogglePhotoMode
  (bind _output_get (LocalVariables|SetEnable (not (Variables|State|GetPhotoModeActive))))
  (Variables|State|SetPhotoModeActive _output_get)
  (if (and (not (LocalVariables|GetEnable)) (Variables|State|GetSelfieModeActive))
    (State|ToggleSelfieMode))
  (Variables|/Script/Engine.SpringArmComponent|SetTargetArmLength (Variables|Default|GetSpringArm) (Math|Float|SelectFloat (Variables|SpringArm|GetPhotoModeSpringArmLength) (Variables|SpringArm|GetDefaultSpringArmLength) (LocalVariables|GetEnable)))
  (Collision|SetCollisionResponsetoAllChannels (Variables|Default|GetCollisionBox) (select (LocalVariables|GetEnable) "ECR_Overlap" "ECR_Ignore"))
  (Components|Box|SetBoxExtent (Variables|Default|GetCollisionBox) (Math|Vector|MakeVector (Variables|/Script/Engine.SpringArmComponent|GetTargetArmLength (Variables|Default|GetSpringArm)) 1e+02 1e+02) true)
  (Variables|/Script/Engine.SpringArmComponent|SetbDoCollisionTest (Variables|Default|GetSpringArm) (not (LocalVariables|GetEnable)))
  (Utilities|IsValid (Variables|UI|GetHUD)
    (:Is%20Valid
      (Default|EnableCameraUI (Variables|UI|GetHUD) (LocalVariables|GetEnable) :!label _label)
      (if (LocalVariables|GetEnable)
        (bind _asplayer_controller (Utilities|Casting|CastToPlayerController (Pawn|GetController (Variables|Owner|GetOwningActor)))
          (:then
            (Input|AddMappingContext (PlayerController|LocalPlayerSubsystems|GetEnhancedInputLocalPlayerSubsystem _asplayer_controller) (Variables|Input|GetInputMappingContext) 1 "(bIgnoreAllPressedKeysUntilRelease=True,bForceImmediately=False)"))
          (:CastFailed
            (Development|PrintString "WARNING: No valid player controller found" true true "(R=1.000000,G=0.018362,B=0.000000,A=1.000000)")))
        (else
          (Camera|SetCameraFOV (Variables|Camera|GetDefaultFOV))
          (bind _asplayer_controller_2 (Utilities|Casting|CastToPlayerController (Pawn|GetController (Variables|Owner|GetOwningActor)))
            (:then
              (Input|RemoveMappingContext (PlayerController|LocalPlayerSubsystems|GetEnhancedInputLocalPlayerSubsystem _asplayer_controller_2) (Variables|Input|GetInputMappingContext) "(bIgnoreAllPressedKeysUntilRelease=True,bForceImmediately=False)"))
            (:CastFailed
              (Development|PrintString "WARNING: No valid player controller found" true true "(R=1.000000,G=0.018362,B=0.000000,A=1.000000)"))))))
    (:Is%20Not%20Valid
      (bind (_success _hud) (CallFunction|GetHUD self))
      (if _success
        (Variables|UI|SetHUD _hud)
        (goto _label)))))

(fn ToggleSelfieMode
  (bind _springarm (Variables|Default|GetSpringArm))
  (bind _relativerotation (Variables|/Script/Engine.SceneComponent|GetRelativeRotation _springarm))
  (bind _output_get (LocalVariables|SetEnable (not (Variables|State|GetSelfieModeActive))))
  (bind _output_get_2 (Variables|State|SetSelfieModeActive _output_get))
  (if _output_get_2
    (Variables|SpringArm|SetPrevSpringArmLength (Variables|/Script/Engine.SpringArmComponent|GetTargetArmLength (Variables|Default|GetSpringArm))))
  (Variables|/Script/Engine.SpringArmComponent|SetTargetArmLength (Variables|Default|GetSpringArm) (Math|Float|SelectFloat (Variables|SpringArm|GetDefaultSpringArmLength) (Variables|SpringArm|GetPrevSpringArmLength) (LocalVariables|GetEnable)))
  (Variables|/Script/Engine.SpringArmComponent|SetbUsePawnControlRotation (Variables|Default|GetSpringArm) (not (LocalVariables|GetEnable)))
  (Transformation|SetRelativeRotation _springarm (Math|Rotator|MakeRotator (.roll _relativerotation) (.pitch _relativerotation) (Math|Float|SelectFloat 1.8e+02 0.0 (LocalVariables|GetEnable))) false false)
  (Variables|Camera|SetDefaultSelfieCamRotation (Variables|/Script/Engine.SceneComponent|GetRelativeRotation (Variables|Default|GetSpringArm)))
  (Input|SetIgnoreMoveInput (Game|GetPlayerController 0) (LocalVariables|GetEnable))
  (return true))

(fn StandardCameraMovement
  (params (ActionValue :type Vector%202D%20Structure))
  (bind _returnvalue (Class|KismetMathLibrary|ClampAxes2D ActionValue -1.0 1.0))
  (bind _standardspeedmultiplier (Variables|Movement|GetStandardSpeedMultiplier))
  (bind _returnvalue_2 (* _returnvalue _standardspeedmultiplier))
  (Pawn|Input|AddControllerYawInput (Variables|Owner|GetOwningActor) (.x _returnvalue_2))
  (Pawn|Input|AddControllerPitchInput (Variables|Owner|GetOwningActor) (* (.y _returnvalue_2) -1.0)))

(fn SelfieCameraMovement
  (params (ActionValue :type Vector%202D%20Structure))
  (bind _defaultselfiecamrotation (Variables|Camera|GetDefaultSelfieCamRotation))
  (bind _defaultselfiecamrotation_2 (Variables|Camera|GetDefaultSelfieCamRotation))
  (bind _selfiemodemaxtilt (Variables|Rotation|GetSelfieModeMaxTilt))
  (bind _springarm (Variables|Default|GetSpringArm))
  (bind _selfiemodemaxrotation (Variables|Rotation|GetSelfieModeMaxRotation))
  (bind _relativerotation (Variables|/Script/Engine.SceneComponent|GetRelativeRotation _springarm))
  (LocalVariables|SetClampedActionValue (Class|KismetMathLibrary|ClampAxes2D ActionValue -1.0 1.0))
  (Transformation|SetRelativeRotation (Variables|Default|GetSpringArm) (Math|Interpolation|RInterpTo (Variables|/Script/Engine.SceneComponent|GetRelativeRotation _springarm) (Math|Rotator|MakeRotator (.roll _relativerotation) (Math|Float|ClampAngle (+ (.pitch _relativerotation) (.y (Movement|GetSelfieCamRotationModifiers (LocalVariables|GetClampedActionValue)))) (- (.pitch _defaultselfiecamrotation_2) _selfiemodemaxtilt) (+ (.pitch _defaultselfiecamrotation_2) _selfiemodemaxtilt)) (Math|Float|ClampAngle (+ (.yaw _relativerotation) (.x (Movement|GetSelfieCamRotationModifiers (LocalVariables|GetClampedActionValue)))) (- (.yaw _defaultselfiecamrotation) _selfiemodemaxrotation) (+ (.yaw _defaultselfiecamrotation) _selfiemodemaxrotation))) (Utilities|Time|GetWorldDeltaSeconds) 5.0) false false))

(fn SetCameraFOV
  (params (NewFOV :type Float%20%28double-precision%29))
  (Camera|SetFieldOfView (Variables|Default|GetCamera) NewFOV)
  (Variables|/Script/Engine.SceneCaptureComponent2D|SetFOVAngle (Variables|Default|GetCameraCaptureComponent) NewFOV))

(fn GetSelfieCamRotationModifiers
  (params (ClampedActionValue :type Vector%202D%20Structure))
  (bind _selfiemodespeedmultiplier (Variables|Movement|GetSelfieModeSpeedMultiplier))
  (bind _returnvalue (* ClampedActionValue _selfiemodespeedmultiplier))
  (return (Math|Vector2D|MakeVector2D (Math|Float|SelectFloat 0.0 (.x _returnvalue) (Math|Float|NearlyEqual(Float) (.x ClampedActionValue) 0.0 0.5)) (Math|Float|SelectFloat 0.0 (.y _returnvalue) (Math|Float|NearlyEqual(Float) (.y ClampedActionValue) 0.0 0.5)))))

(fn MoveCamera
  (params (ActionValue :type Vector%202D%20Structure))
  (if (Variables|State|GetSelfieModeActive)
    (Movement|SelfieCameraMovement ActionValue)
    (else
      (Movement|StandardCameraMovement ActionValue))))

(fn ZoomCamera
  (params (ActionValue :type Float%20%28double-precision%29))
  (bind _returnvalue (Movement|GetBoomHeightAlpha))
  (bind _springarm (Variables|Default|GetSpringArm))
  (bind _defaultspringarmlength (Variables|SpringArm|GetDefaultSpringArmLength))
  (bind _collisionbox (Variables|Default|GetCollisionBox))
  (bind _collisionbox_2 (Variables|Default|GetCollisionBox))
  (bind _camera (Variables|Default|GetCamera))
  (bind _returnvalue_2 (Components|Box|GetUnscaledBoxExtent _collisionbox_2))
  (bind _returnvalue_3 (* _defaultspringarmlength 2.5))
  (bind _returnvalue_4 (* _defaultspringarmlength 0.5))
  (bind _fieldofview (Variables|/Script/Engine.CameraComponent|GetFieldOfView _camera))
  (bind _relativelocation (Variables|/Script/Engine.SceneComponent|GetRelativeLocation _springarm))
  (bind _relativelocation_2 (Variables|/Script/Engine.SceneComponent|GetRelativeLocation _collisionbox))
  (bind _returnvalue_5 (Math|Float|Lerp _returnvalue_4 _returnvalue_3 _returnvalue))
  (if (Variables|State|GetPhotoModeActive)
    (Camera|SetCameraFOV (Math|Interpolation|FInterpTo _fieldofview (Math|Float|Clamp(Float) (+ _fieldofview (* ActionValue (Variables|Zoom|GetCameraZoomMultiplier) -1.0)) (Variables|Camera|GetMaxZoomFOV) (Variables|Camera|GetDefaultFOV)) (Utilities|Time|GetWorldDeltaSeconds) (Variables|Zoom|GetCameraZoomLerpSpeed)))
    (Transformation|SetRelativeLocation _springarm (Math|Vector|MakeVector (.x _relativelocation) (.y _relativelocation) (Math|Float|Lerp (Variables|SpringArm|GetDefaultSpringArmHeight) (Variables|SpringArm|GetMaxSpringArmHeight) (Movement|GetBoomHeightAlpha))) false false)
    (Components|Box|SetBoxExtent _collisionbox_2 (Math|Vector|MakeVector _returnvalue_5 (.y _returnvalue_2) (.z _returnvalue_2)) true)
    (Transformation|SetRelativeLocation (Variables|Default|GetCollisionBox) (Math|Vector|MakeVector (/ _returnvalue_5 2.0) (.y _relativelocation_2) (.z _relativelocation_2)) false false)))

(fn GetBoomHeightAlpha
  (return (- 1.0 (/ (- (Variables|/Script/Engine.CameraComponent|GetFieldOfView (Variables|Default|GetCamera)) (Variables|Camera|GetMaxZoomFOV)) (- (Variables|Camera|GetDefaultFOV) (Variables|Camera|GetMaxZoomFOV))))))

(fn TakePhoto
  (bind _returnvalue (Rendering|CreateRenderTarget2D 1920 1080 "RTF_RGBA8_SRGB"))
  (Variables|/Script/Engine.SceneCaptureComponent2D|SetTextureTarget (Variables|Default|GetCameraCaptureComponent) _returnvalue)
  (Rendering|SceneCapture|CaptureScene (Variables|Default|GetCameraCaptureComponent) :!class /Script/Engine.SceneCaptureComponent2D)
  (Utilities|IsValid (Variables|UI|GetHUD)
    (:Is%20Valid
      (Default|EnablePhotoConfirmationUI (Variables|UI|GetHUD) true (Variables|/Script/Engine.SceneCaptureComponent2D|GetTextureTarget (Variables|Default|GetCameraCaptureComponent)) (Variables|GalleryManager|GetPhotoGalleryManager) :!label _label))
    (:Is%20Not%20Valid
      (bind (_success _hud) (CallFunction|GetHUD self))
      (if _success
        (Variables|UI|SetHUD _hud)
        (goto _label)))))

(fn SetGalleryManager
  (params (IN_PhotoGalleryManager :type BP%20Photo%20Gallery%20Manager%20Object%20Reference))
  (Variables|GalleryManager|SetPhotoGalleryManager IN_PhotoGalleryManager))

(fn TogglePhotoGallery
  (params (Enable :type Boolean))
  (bind _photogallerymanager (Variables|GalleryManager|GetPhotoGalleryManager)
    (:then
      (Default|TogglePhotoGallery _photogallerymanager Enable)
      (Variables|State|SetPhotographyDisabled Enable)
      (Input|SetIgnoreMoveInput (Pawn|GetController (Variables|Owner|GetOwningActor)) false))
    (:else)))

(fn DisablePhotography
  (params (Disable :type Boolean))
  (Variables|State|SetPhotographyDisabled Disable))

(fn BoxCollisionBeginOverlap
  (params (OverlappedComponent :type Primitive%20Component%20Object%20Reference) (OtherActor :type Actor%20Object%20Reference) (OtherComp :type Primitive%20Component%20Object%20Reference) (OtherBodyIndex :type Integer) (bFromSweep :type Boolean) (SweepResult :type Hit%20Result%20Structure%20%28by%20ref%29))
  (bind _asbp_item_base (Utilities|Casting|CastToBP_ItemBase OtherActor))
  (if (Controller|LineOfSightTo (Pawn|GetController (Variables|Owner|GetOwningActor)) _asbp_item_base "0, 0, 0" false)
    (Utilities|Array|AddUnique (Variables|ItemIdentification|GetItemsInRange) (Variables|/Game/Blueprints/Items/BP_ItemBase.BP_ItemBase_C|GetItemID _asbp_item_base))
    (Development|PrintString (Utilities|String|ToString(Name) (Variables|/Game/Blueprints/Items/BP_ItemBase.BP_ItemBase_C|GetItemID _asbp_item_base)) true true "(R=1.000000,G=0.302545,B=0.000000,A=1.000000)")
    (return)))

(fn InitialiseBoxCollision
  (bind _returnvalue (Game|AddComponentbyClass (Variables|Owner|GetOwningActor) "/Script/Engine.BoxComponent" true))
  (bind _output_get (Variables|Default|SetCollisionBox _returnvalue))
  (Collision|SetCollisionResponsetoAllChannels _output_get "ECR_Ignore")
  (Components|Box|SetBoxExtent (Variables|Default|GetCollisionBox) (Math|Vector|MakeVector (* (Variables|SpringArm|GetDefaultSpringArmLength) 0.5) 1.5e+02 1.5e+02) true)
  (Transformation|AttachComponentToComponent (Variables|Default|GetCollisionBox) (Variables|Default|GetSpringArm) "None" "SnapToTarget" "SnapToTarget" "KeepRelative" true)
  (Transformation|SetRelativeLocation (Variables|Default|GetCollisionBox) (Math|Vector|MakeVector (/ (Variables|SpringArm|GetDefaultSpringArmLength) 2.0) 0.0 0.0) false false)
  (Collision|BindEventtoOnComponentBeginOverlap (Variables|Default|GetCollisionBox) (EventDispatchers|CreateEvent :!event BoxCollisionBeginOverlap))
  (Collision|BindEventtoOnComponentEndOverlap (Variables|Default|GetCollisionBox) (EventDispatchers|CreateEvent :!event BoxCollisionEndOverlap))
  (Development|SetHiddeninGame (Variables|Default|GetCollisionBox) false false)
  (Class|BoxComponent|SetLineThickness (Variables|Default|GetCollisionBox) 2.0))

(fn BoxCollisionEndOverlap
  (params (OverlappedComponent :type Primitive%20Component%20Object%20Reference) (OtherActor :type Actor%20Object%20Reference) (OtherComp :type Primitive%20Component%20Object%20Reference) (OtherBodyIndex :type Integer)))