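; BP_ItemBase is an item Blueprint that sets its static mesh from data.
; Its construction script looks up ItemID as a row in DT_Items and applies that row's StaticMesh to the SMBase component.
; The lookup runs only when OverrideDefaultStaticMesh is off and ItemID is not empty.
; A missing row prints a warning that names the ID.
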(fn ConstructionScript
  (if (Math|Boolean|NORBoolean (Variables|Default|GetOverrideDefaultStaticMesh) (Utilities|Array|IsEmpty (Utilities|String|ToString(Name) (Variables|Default|GetItemID))))
    (bind _returnvalue (Utilities|GetDataTableRow "/Game/Blueprints/Items/Data/DT_Items.DT_Items" (Variables|Default|GetItemID))
      (:then
        (Components|StaticMesh|SetStaticMesh (Variables|Default|GetSM_Base) (.StaticMesh (Utilities|Struct|BreakFItemData _returnvalue))))
      (:RowNotFound
        (Development|PrintString (Utilities|String|Append "WARNING: Cannot find item " (Utilities|String|ToString(Name) (Variables|Default|GetItemID)) " in Data Table. "))))))